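; AirPlane is a drop plane that carries the player's view across the map until the player jumps out.
; On BeginPlay it shows a JumpUMG widget and runs a timeline that lerps it along a fixed diagonal at constant altitude, setting itself as view target every update.
; Mouse input orbits and zooms its spring arm.
; The widget's jump dispatcher or timeline end destroys it, moving the player character to its location and rotation.
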(event Custom|CustomEvent_0
  (Actor|DestroyActor))

(event EventBeginPlay
  (Utilities|FlowControl|Sequence
    (:then_0
      (bind _returnvalue (UserInterface|CreateWidget "/Game/HotBlood/Blueprints/LW_BP/JumpUMG.JumpUMG_C"))
      (UserInterface|Viewport|AddtoViewport _returnvalue 0)
      (EventDispatchers|BindEventtoJumpDisp _returnvalue (delegate Custom|CustomEvent_0)))
    (:then_1
      (bind _alpha (Timeline|Timeline_0 PlayFromStart)
        (:Update
          (Transformation|SetActorLocation (Math|Vector|Lerp(Vector) "-200000.000000,-200000.000000,50000.000000" "200000.000000,200000.000000,50000.000000" _alpha) false false)
          (Game|Player|SetViewTargetwithBlend (Game|GetPlayerController 0) self 0.0 "VTBlend_Cubic" 0.0 false))
        (:Finished
          (Actor|DestroyActor))))))

(event EventTick
  (params (DeltaSeconds :type Float%20%28single-precision%29)))

(event EventDestroyed
  (bind _returnvalue (Transformation|GetActorTransform))
  (bind (_location _rotation) (Math|Transform|BreakTransform _returnvalue))
  (Transformation|SetActorTransform (Game|GetPlayerCharacter 0) (Math|Transform|MakeTransform _location _rotation)))

(event Input|AxisEvents|InputAxisLookUp
  (params (AxisValue :type Float%20%28single-precision%29))
  (bind _springarm (Variables|Default|GetSpringArm))
  (bind _relativerotation (Variables|/Script/Engine.SceneComponent|GetRelativeRotation _springarm))
  (bind (_roll _pitch _yaw) (Math|Rotator|BreakRotator _relativerotation))
  (Transformation|SetRelativeRotation (Variables|Default|GetSpringArm) (Math|Rotator|MakeRotator _roll (Math|Float|Clamp(Float) (+ _pitch (* AxisValue -2.0)) -4e+01 4e+01) _yaw) false false))

(event Input|AxisEvents|InputAxisTurn
  (params (AxisValue :type Float%20%28single-precision%29))
  (bind _springarm (Variables|Default|GetSpringArm))
  (bind _relativerotation (Variables|/Script/Engine.SceneComponent|GetRelativeRotation _springarm))
  (bind (_roll _pitch _yaw) (Math|Rotator|BreakRotator _relativerotation))
  (Transformation|SetRelativeRotation (Variables|Default|GetSpringArm) (Math|Rotator|MakeRotator _roll _pitch (+ (* AxisValue 2.0) _yaw)) false false))

(event Input|MouseEvents|MouseWheelAxis
  (params (AxisValue :type Float%20%28single-precision%29))
  (bind _springarm (Variables|Default|GetSpringArm))
  ;[1 1 1] 中间滚轮
  (Variables|/Script/Engine.SpringArmComponent|SetTargetArmLength _springarm (+ (Variables|/Script/Engine.SpringArmComponent|GetTargetArmLength _springarm) (* AxisValue -5e+01))))

(fn ConstructionScript)